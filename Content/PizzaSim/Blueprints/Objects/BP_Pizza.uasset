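; BP_Pizza is the pizza object for the pizza sim, with topping and box components that start out hidden.
; On BeginPlay it hides the Pepperoni, Sweetcorn and PizzaBox components.
; ChangeMaterial gives the Sphere component a dynamic instance of M_Concrete_Grime as the cooked look, but nothing in this Blueprint calls it.
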(event EventBeginPlay
  (CallFunction|SetDefaultInvisibleComponents))

(event Collision|EventActorBeginOverlap
  (params (OtherActor :type Actor%20Object%20Reference)))

(event EventTick
  (params (DeltaSeconds :type Float%20%28single-precision%29)))

(fn ConstructionScript)

(fn ChangeMaterial
  ;[1 1 1] Change material of pizza when cooked
  (Rendering|Material|CreateDynamicMaterialInstance (Variables|Default|GetSphere) 0 "/Game/StarterContent/Materials/M_Concrete_Grime.M_Concrete_Grime" "None" :!class /Script/Engine.PrimitiveComponent))

(fn SetDefaultInvisibleComponents
  ;[1 1 1] Set toppings invisible
  (Rendering|SetVisibility (Variables|Default|GetPepperoni) false false)
  (Rendering|SetVisibility (Variables|Default|GetSweetcorn) false false)
  (Rendering|SetVisibility (Variables|Default|GetPizzaBox) false false))