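; BP_Customer is an AI pizza-shop customer with a hard-coded order for a cooked pepperoni and sweetcorn pizza.
; On BeginPlay it stores the player in its controller's blackboard.
; Tick polls the player's FoodIsServed flag, then either pays for a matching order or prints a frustration message and clears the flag.
; Either outcome sets the blackboard Leave bool so the AI leaves; PizzaIsServed is an empty stub.
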(event EventBeginPlay
  (bind _asbp_customer_controller (Utilities|Casting|CastToBP_CustomerController (AI|GetAIController 0)))
  (AI|Components|Blackboard|SetValueasObject (AI|GetBlackboard _asbp_customer_controller) (Variables|Default|Getplayer) (Game|GetPlayerCharacter 0)))

(event Collision|EventActorBeginOverlap
  (params (OtherActor :type Actor%20Object%20Reference)))

(event EventTick
  (params (DeltaSeconds :type Float%20%28single-precision%29))
  (bind _asbp_player_character (Utilities|Casting|CastToBP_PlayerCharacter (Game|GetPlayerCharacter 0)))
  (if (Variables|/Game/PizzaSim/Blueprints/Player/BP_PlayerCharacter.BP_PlayerCharacter_C|GetfoodIsServed _asbp_player_character)
    (if (Math|Boolean|ANDBoolean (Variables|/Game/PizzaSim/Blueprints/Player/BP_PlayerCharacter.BP_PlayerCharacter_C|Getcooked _asbp_player_character) (Variables|/Game/PizzaSim/Blueprints/Player/BP_PlayerCharacter.BP_PlayerCharacter_C|Getsweetcorn _asbp_player_character) (Variables|/Game/PizzaSim/Blueprints/Player/BP_PlayerCharacter.BP_PlayerCharacter_C|Getpepperoni _asbp_player_character))
      (Default|GetPaid _asbp_player_character)
      (else
        (CallFunction|DontPay _asbp_player_character)))
    (CallFunction|LeaveShop (AI|GetAIController 0))))

(fn ConstructionScript)

(fn PizzaIsServed)

(fn LeaveShop
  (params (Object :type Object%20Object%20Reference))
  ;[1 1 1] Set bool to leave so AI leaves shop
  (bind _asbp_customer_controller (Utilities|Casting|CastToBP_CustomerController Object))
  (AI|Components|Blackboard|SetValueasBool (AI|GetBlackboard _asbp_customer_controller) (Variables|Default|Getleave) true))

(fn DontPay
  (params (player :type BP%20Player%20Character%20Object%20Reference))
  (Development|PrintString "CUSTOMER LEFT IN FRUSTRATION" true true "(R=1.000000,G=0.000000,B=0.249370,A=1.000000)")
  (Variables|/Game/PizzaSim/Blueprints/Player/BP_PlayerCharacter.BP_PlayerCharacter_C|SetfoodIsServed player false))