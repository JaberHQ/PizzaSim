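; Player character for a pizza sim that picks up a pizza and places it in an oven with a single PickUp input.
; A camera-forward line trace finds a pizza to attach to the mesh's holding socket or, when already holding, an oven to attach it to.
; An IsHolding flag switches between the two actions.
; Baking is only a fixed delay between debug prints, with no change to the pizza.
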(event EventBeginPlay)

(event Collision|EventActorBeginOverlap
  (params (OtherActor :type Actor%20Object%20Reference)))

(event EventTick
  (params (DeltaSeconds :type Float%20%28single-precision%29)))

(event Input|ActionEvents|InputActionPickUp
  (params (Key :type Key%20Structure :default "None"))
  (bind _cameracomp (Variables|Default|GetcameraComp))
  (bind _cameracomp_2 (Variables|Default|GetcameraComp))
  (bind _returnvalue (Transformation|GetWorldLocation _cameracomp_2))
  (bind _returnvalue_2 (Transformation|GetWorldLocation _cameracomp))
  (:Pressed
    (if (Variables|Default|GetisHolding)
      (bind (_outhit _returnvalue_3) (Collision|LineTraceByChannel _returnvalue_2 (+ _returnvalue_2 (* (Math|Vector|GetForwardVector _cameracomp) (Variables|Default|GettraceLength))) "TraceTypeQuery2" false 0 "ForDuration"))
      (if _returnvalue_3
        (bind _asbp_oven (Utilities|Casting|CastToBP_Oven (.HitActor (Collision|BreakHitResult _outhit))))
        (Transformation|AttachActorToActor (Variables|Default|GetAs%20BP%20Pizza) _asbp_oven "None" "SnapToTarget" "KeepWorld" "KeepWorld" true)
        (Variables|Default|SetisHolding false)
        (Development|PrintString "PIZZA IS IN THE OVEN")
        (Utilities|FlowControl|Delay 5.0)
        (Development|PrintString "Pizza is done"))
      (else
        (bind (_outhit_2 _returnvalue_4) (Collision|LineTraceByChannel _returnvalue (+ _returnvalue (* (Math|Vector|GetForwardVector _cameracomp_2) (Variables|Default|GettraceLength))) "TraceTypeQuery2" false 0 "ForDuration"))
        (if _returnvalue_4
          (bind _asbp_pizza (Utilities|Casting|CastToBP_Pizza (.HitActor (Collision|BreakHitResult _outhit_2))))
          (bind _output_get (Variables|Default|SetAs%20BP%20Pizza _asbp_pizza))
          (Development|PrintString "PUT PIZZA IN THE OVEN")
          (Transformation|AttachComponentToComponent _output_get (Variables|Character|GetMesh) "HoldingSocket" "KeepWorld" "KeepWorld" "KeepWorld" true)
          (Variables|Default|SetisHolding true))))))

(fn ConstructionScript)